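; Secondary character actor that appears as one of four personas (ShockGirl, BigLady, LumberJackMan, OldMan) and supplies a player animation status and happiness change.
; BeginPlay picks the persona at random and sets the matching Paper2D flipbook.
; GetPlayerAnimStatus maps the persona to both outputs, with an InvertChance percentage roll that flips the reaction for ShockGirl and LumberJackMan only.
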(event EventBeginPlay
  (switch int (Math|Random|RandomIntegerinRange 1 4)
    (:1
      (Variables|Default|SetCharacterIdent "NewEnumerator0"))
    (:2
      (Variables|Default|SetCharacterIdent "NewEnumerator1"))
    (:3
      (Variables|Default|SetCharacterIdent "NewEnumerator2"))
    (:4
      (Variables|Default|SetCharacterIdent "NewEnumerator3")))
  (Sprite|SetFlipbook (Variables|Default|GetSprite) (Utilities|Select :Index (Variables|Default|GetCharacterIdent) :NewEnumerator0 (Variables|Skin|GetShockGirl) :NewEnumerator1 (Variables|Skin|GetFatLadyAnimation) :NewEnumerator2 (Variables|Skin|GetLumberJack) :NewEnumerator3 (Variables|Skin|GetOldManAnimation))))

(fn ConstructionScript)

(fn GetPlayerAnimStatus
  (bind _characterident (Variables|Default|GetCharacterIdent))
  (bind _characterident_2 (Variables|Default|GetCharacterIdent))
  (if (or (Utilities|Enum|Equal(Enum) _characterident "NewEnumerator0") (Utilities|Enum|Equal(Enum) _characterident "NewEnumerator2"))
    (if (< (Math|Random|RandomIntegerinRange 0 100) (Variables|Default|GetInvertChance))
      (return (Utilities|Select :Index _characterident_2 :NewEnumerator0 "NewEnumerator8" :NewEnumerator1 "NewEnumerator2" :NewEnumerator2 "NewEnumerator7" :NewEnumerator3 "NewEnumerator4") (Utilities|Select :Index _characterident_2 :NewEnumerator0 5e+01 :NewEnumerator1 0.0 :NewEnumerator2 -3e+01 :NewEnumerator3 -15.0))
      (else
        _)))
  (bind _output_get (Variables|Default|SetHappinesfeedback (Utilities|Select :Index _characterident :NewEnumerator0 -3e+01 :NewEnumerator1 15.0 :NewEnumerator2 15.0 :NewEnumerator3 -15.0)))
  (return (Utilities|Select :Index _characterident :NewEnumerator0 "NewEnumerator3" :NewEnumerator1 "NewEnumerator2" :NewEnumerator2 "NewEnumerator6" :NewEnumerator3 "NewEnumerator4") _output_get))